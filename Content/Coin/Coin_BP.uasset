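; Collectible coin actor that adds to the player's score when picked up.
; Tick plays the UpDown timeline, which lerps the static mesh's relative Z position for a vertical hover motion.
; When a ThirdPersonCharacter begins overlapping the Box, the coin increments that character's Score variable directly and destroys itself.
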(event `self.ReceiveTick`
  (params (DeltaSeconds :type "Float (single-precision)"))
  (bind (_direction _up___down_movement) (`Timeline|Up & Down`)
    (:`Update`
      (`SceneComponent.K2_SetRelativeLocation` (`self.StaticMesh`) (`KismetMathLibrary.VLerp` (0.0 0.0 80.0) (0.0 0.0 110.0) _up___down_movement) false false))))

(event `self.Box.OnComponentBeginOverlap`
  (params (OverlappedComponent :type "PrimitiveComponent Object Reference") (OtherActor :type "Actor Object Reference") (OtherComp :type "PrimitiveComponent Object Reference") (OtherBodyIndex :type Integer) (bFromSweep :type Boolean) (SweepResult :type "HitResult Structure (by ref)"))
  ;[1 1 1] Colect coins
  (bind _asthird_person_character (cast `/Game/ThirdPersonBP/Blueprints/ThirdPersonCharacter` OtherActor))
  (bind _output_get (set `self.TPCharacter` _asthird_person_character))
  (bind _result (`/Engine/EditorBlueprintResources/StandardMacros.IncrementInt` (`/Game/ThirdPersonBP/Blueprints/ThirdPersonCharacter.Score` _output_get))
    (:`  `
      (set `/Game/ThirdPersonBP/Blueprints/ThirdPersonCharacter.Score` _result _output_get)
      (`self.K2_DestroyActor`))))

(fn `UserConstructionScript`)