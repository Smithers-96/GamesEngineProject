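; Puzzle01_bp is a floor pad for the first room puzzle that toggles on and off, Lights Out style, when stepped on.
; A ThirdPersonCharacter overlapping its Box flips IsOn on itself and on every pad in AdjacentPads.
; Tick sets the Cube material from IsOn every frame.
; When an overlap ends while the pad is on, the Box is destroyed, so only neighboring pads can toggle it afterward.
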(event `self.ReceiveTick`
  (params (DeltaSeconds :type "Float (single-precision)"))
  (bind _cube (`self.Cube`))
  ;[1 1 1] When the player touches the pads, it will be assigned to different colours
  (if (`self.IsOn?`)
    (`PrimitiveComponent.SetMaterial` _cube 0 "/Game/Puzzle/FirstRoomPuzzle/isOn.isOn")
    (else
      (`PrimitiveComponent.SetMaterial` _cube 0 "/Game/Puzzle/FirstRoomPuzzle/isOff.isOff"))))

(event `self.Box.OnComponentBeginOverlap`
  (params (OverlappedComponent :type "PrimitiveComponent Object Reference") (OtherActor :type "Actor Object Reference") (OtherComp :type "PrimitiveComponent Object Reference") (OtherBodyIndex :type Integer) (bFromSweep :type Boolean) (SweepResult :type "HitResult Structure (by ref)"))
  ;[1 1 1] Begin box collision when player steps on it
  (if (== (`GameplayStatics.GetObjectClass` OtherActor) "/Game/ThirdPersonBP/Blueprints/ThirdPersonCharacter.ThirdPersonCharacter_C")
    (if (`self.IsOn?`)
      (set `self.IsOn?` false)
      (else
        (set `self.IsOn?` true)))
    (for _array_element (`self.AdjacentPads`)
      (if (`/Game/Puzzle/FirstRoomPuzzle/Puzzle01_bp.IsOn?` _array_element)
        (set `/Game/Puzzle/FirstRoomPuzzle/Puzzle01_bp.IsOn?` false _array_element)
        (else
          (set `/Game/Puzzle/FirstRoomPuzzle/Puzzle01_bp.IsOn?` true _array_element))))))

(event `self.Box.OnComponentEndOverlap`
  (params (OverlappedComponent :type "PrimitiveComponent Object Reference") (OtherActor :type "Actor Object Reference") (OtherComp :type "PrimitiveComponent Object Reference") (OtherBodyIndex :type Integer))
  ;[1 1 1] End Box Collision on tiles when player steps on it
  (if (`self.IsOn?`)
    (`ActorComponent.K2_DestroyComponent` (`self.Box`))))

(fn `UserConstructionScript`)