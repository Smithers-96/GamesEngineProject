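; Pads_bp is an unfinished manager Blueprint for the nine pads of the first room puzzle.
; Tick feeds a Gate whose exit loops over PadsArray and casts each entry to Pad_child, with no further action.
; The node filling that array from the individual pad variables is disconnected, and the pads' IsOn read is unused, so no puzzle logic takes effect.
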(event `self.ReceiveTick`
  (params (DeltaSeconds :type "Float (single-precision)"))
  (`/Engine/EditorBlueprintResources/StandardMacros.Gate` true
    (:`Exit`
      (for _ (`self.pads_array`)
        (bind _aspad_child (cast `/Game/Puzzle/FirstRoomPuzzle/Pad_child` _))))))

(fn `UserConstructionScript`)